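; BP_TapePawn is a pawn that selects which of its two cameras is active based on the running platform.
; On BeginPlay it activates WindowsCamera and deactivates Camera when the platform name is Windows.
; On every other platform it activates Camera and deactivates WindowsCamera instead.
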(event EventBeginPlay
  (if (Utilities|Enum|Equal(Enum) (Game|GetPlatformName) "Windows")
    (Components|Activation|Activate (Variables|Default|GetWindowsCamera) false)
    (Components|Activation|Deactivate (Variables|Default|GetCamera))
    (else
      (Components|Activation|Activate (Variables|Default|GetCamera) false)
      (Components|Activation|Deactivate (Variables|Default|GetWindowsCamera)))))

(fn ConstructionScript)