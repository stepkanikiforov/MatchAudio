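; Discography actor that scrolls vertically in the world as a finger drags on the screen.
; Tick polls Touch1, latches the starting Y once per press through a DoOnce reset on release, then turns each frame's Y delta into a Z move scaled by SpeedMovement and delta time.
; The new height is clamped between zero and the negated Border value, so Border is expected to be negative.
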(event EventTick
  (params (DeltaSeconds :type Float%20%28single-precision%29))
  (bind _returnvalue (Game|GetPlayerController 0))
  (bind _self self)
  (bind _border (Variables|Default|GetBorder))
  (bind (_locationx _locationy _biscurrentlypressed) (Class|PlayerController|GetInputTouchState _returnvalue "Touch1"))
  (bind _returnvalue_2 (* -1 _border))
  (bind _returnvalue_3 (Transformation|GetActorLocation _self))
  (if _biscurrentlypressed
    (Utilities|FlowControl|Sequence
      (:then_0
        (Utilities|FlowControl|DoOnce false :!label _label
          (:Completed
            (Variables|Default|SetStartLocation _locationy))))
      (:then_1
        (bind _output_get (Variables|Default|SetFinishLocation _locationy))
        (bind _output_get_2 (Variables|Default|SetDelta (- _output_get (Variables|Default|GetStartLocation))))
        (if (!= _output_get_2 0.0)
          (if (>= (- (.z _returnvalue_3) (* (* (Variables|Default|GetDelta) (Variables|Default|GetSpeedMovement)) DeltaSeconds)) _returnvalue_2)
            (Variables|Default|SetLocationToSet _returnvalue_2)
            (elif (<= (- (.z _returnvalue_3) (* (* (Variables|Default|GetDelta) (Variables|Default|GetSpeedMovement)) DeltaSeconds)) 0.0)
              (Variables|Default|SetLocationToSet 0.0)
              (else
                (Variables|Default|SetLocationToSet (- (.z _returnvalue_3) (* (* (Variables|Default|GetDelta) (Variables|Default|GetSpeedMovement)) DeltaSeconds))))))
          (Transformation|SetActorLocation _self (Math|Vector|MakeVector (.x _returnvalue_3) (.y _returnvalue_3) (Variables|Default|GetLocationToSet)) false false)
          (Variables|Default|SetStartLocation (Variables|Default|GetFinishLocation)))))
    (else
      (goto _label Reset))))

(fn ConstructionScript)