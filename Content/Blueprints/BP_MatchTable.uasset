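; BP_MatchTable is the match table actor that relays scoring events to BP_MatchAudioGameMode.
; On BeginPlay it binds handlers to its track-destroy, combo-score and single-score delegates.
; Combo events pass combo and type to ShowCombo, while single scores call SetCurrentScore without forwarding score or type.
; The track-destroy handler is bound but empty.
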(event Custom|DestroyTrack
  (params (Track :type Integer)))

(event Custom|ComboScore
  (params (Combo :type Integer) (Type :type Integer))
  (bind _asbp_match_audio_game_mode (Utilities|Casting|CastToBP_MatchAudioGameMode (Game|GetGameMode)))
  (Default|ShowCombo _asbp_match_audio_game_mode Combo Type))

(event Custom|SingleScore
  (params (Score :type Integer) (Type :type Integer))
  (bind _asbp_match_audio_game_mode (Utilities|Casting|CastToBP_MatchAudioGameMode (Game|GetGameMode)))
  (Default|SetCurrentScore _asbp_match_audio_game_mode))

(event EventBeginPlay
  (EventDispatchers|AssignDelegateTrackDestroy (delegate Custom|DestroyTrack))
  (EventDispatchers|AssignDelegateComboScore (delegate Custom|ComboScore))
  (EventDispatchers|AssignDelegateSingleScore (delegate Custom|SingleScore)))

(event Collision|EventActorBeginOverlap
  (params (OtherActor :type Actor%20Object%20Reference)))

(event EventTick
  (params (DeltaSeconds :type Float%20%28single-precision%29)))

(fn ConstructionScript)