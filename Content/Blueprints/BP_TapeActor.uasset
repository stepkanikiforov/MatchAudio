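; BP_TapeActor is a tape actor that labels its widget component, a WBP_DiscographyItem, with a sound name.
; Shortly after BeginPlay, it casts the widget and calls SetSoundName.
; On non-Windows platforms it strips the Android Download folder path and .mp3 extension from the name and passes SoundIndex.
; On Windows it passes the unmodified name with index zero.
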(event EventBeginPlay
  (bind _soundname (Variables|Default|GetSoundName))
  (Utilities|FlowControl|Delay 0.2)
  (bind _aswbp_discography_item (Utilities|Casting|CastToWBP_DiscographyItem (UserInterface|GetWidget (Variables|Default|GetWidget))))
  (if (Utilities|Enum|NotEqual(Enum) (Game|GetPlatformName) "Windows")
    (Default|SetSoundName _aswbp_discography_item (Utilities|String|Replace (Utilities|String|Replace _soundname "/storage/emulated/0/Download/") ".mp3") (Variables|Default|GetSoundIndex))
    (else
      (Default|SetSoundName _aswbp_discography_item _soundname))))

(fn ConstructionScript)