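; Game instance for an FMOD audio-driven game that owns the FMOD manager and the player's total score.
; Init constructs the manager, then binds to app deactivate and enter-background delegates and to the manager's sound-over delegate.
; Losing focus pauses audio analysis, playback and the game, with no resume handled here.
; When a sound ends, it adds the match-audio game mode's current score to the total and saves.
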(event Custom|PauseSound
  (bind _fmodmanager (Variables|Default|GetFMODManager))
  (Utilities|IsValid _fmodmanager
    (:Is%20Valid
      (Class|FMODManager|PauseAnalyze _fmodmanager true)
      (Class|FMODManager|PausePlayer _fmodmanager true)
      (Game|SetGamePaused true))))

(event Custom|OverSound
  (bind _asbp_match_audio_game_mode (Utilities|Casting|CastToBP_MatchAudioGameMode (Game|GetGameMode)))
  (Variables|Default|SetTotalScore (+ (Variables|Default|GetTotalScore) (Variables|/Script/MatchAudio.MatchAudioGameMode|GetCurrentScore _asbp_match_audio_game_mode)))
  (Class|MatchAudioGameInstance|SaveGame))

(event EventInit
  (Utilities|FlowControl|Sequence
    (:then_0
      (bind _returnvalue (Game|ConstructObjectfromClass "/Game/Blueprints/BP_FMODManager.BP_FMODManager_C" self))
      (Variables|Default|SetFMODManager _returnvalue))
    (:then_1
      (EventDispatchers|AssignApplicationWillDeactivateDelegate (delegate Custom|PauseSound))
      (EventDispatchers|AssignApplicationWillEnterBackgroundDelegate (delegate Custom|PauseSound)))
    (:then_2
      (EventDispatchers|AssignDelegateOverSound (Variables|Default|GetFMODManager) (delegate Custom|OverSound)))))